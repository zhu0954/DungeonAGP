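; Dungeon room piece that opens its walls where it adjoins other rooms or corridors.
; Shortly after BeginPlay, a single overlap check reads the colliders on the right, back, front and left walls.
; Each wall switches to the open-wall mesh when its collider overlaps a base room, corridor, statue, loot or enemy room, identified through chained casts.
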(event Collision|EventActorBeginOverlap
  (params (OtherActor :type Actor%20Object%20Reference)))

(event EventTick
  (params (DeltaSeconds :type Float%20%28single-precision%29)))

(event EventBeginPlay
  (Utilities|FlowControl|Delay 0.2)
  (CallFunction|CheckInitialOverlap))

(fn ConstructionScript)

(fn CheckInitialOverlap
  (for _array_element (Collision|GetOverlappingActors (Variables|Default|GetRightWallCollider) 0 :!class /Script/Engine.PrimitiveComponent)
    (Utilities|Casting|CastToBP_BaseRoom _array_element
      (:then
        _)
      (:CastFailed
        (Utilities|Casting|CastToBP_Corridor _array_element
          (:then
            _)
          (:CastFailed
            (Utilities|Casting|CastToBP_StatueRoom _array_element
              (:then
                _)
              (:CastFailed
                (Utilities|Casting|CastToBP_LootRoom _array_element
                  (:then
                    _)
                  (:CastFailed
                    (Utilities|Casting|CastToBP_EnemyRoom _array_element)))))))))
    (Components|StaticMesh|SetStaticMesh (Variables|Default|GetRightWall) "/Game/Blueprints/Dungeon/OpenWallMesh.OpenWallMesh"))
  (for _array_element_2 (Collision|GetOverlappingActors (Variables|Default|GetBackWallCollider) 0 :!class /Script/Engine.PrimitiveComponent)
    (Utilities|Casting|CastToBP_BaseRoom _array_element_2
      (:then
        _)
      (:CastFailed
        (Utilities|Casting|CastToBP_Corridor _array_element_2
          (:then
            _)
          (:CastFailed
            (Utilities|Casting|CastToBP_StatueRoom _array_element_2
              (:then
                _)
              (:CastFailed
                (Utilities|Casting|CastToBP_LootRoom _array_element_2
                  (:then
                    _)
                  (:CastFailed
                    (Utilities|Casting|CastToBP_EnemyRoom _array_element_2)))))))))
    (Components|StaticMesh|SetStaticMesh (Variables|Default|GetBackWall) "/Game/Blueprints/Dungeon/OpenWallMesh.OpenWallMesh"))
  (for _array_element_3 (Collision|GetOverlappingActors (Variables|Default|GetFrontWallCollider) 0 :!class /Script/Engine.PrimitiveComponent)
    (Utilities|Casting|CastToBP_BaseRoom _array_element_3
      (:then
        _)
      (:CastFailed
        (Utilities|Casting|CastToBP_Corridor _array_element_3
          (:then
            _)
          (:CastFailed
            (Utilities|Casting|CastToBP_StatueRoom _array_element_3
              (:then
                _)
              (:CastFailed
                (Utilities|Casting|CastToBP_LootRoom _array_element_3
                  (:then
                    _)
                  (:CastFailed
                    (Utilities|Casting|CastToBP_EnemyRoom _array_element_3)))))))))
    (Components|StaticMesh|SetStaticMesh (Variables|Default|GetFrontWall) "/Game/Blueprints/Dungeon/OpenWallMesh.OpenWallMesh"))
  (for _array_element_4 (Collision|GetOverlappingActors (Variables|Default|GetLeftWallCollider) 0 :!class /Script/Engine.PrimitiveComponent)
    (Utilities|Casting|CastToBP_BaseRoom _array_element_4
      (:then
        _)
      (:CastFailed
        (Utilities|Casting|CastToBP_Corridor _array_element_4
          (:then
            _)
          (:CastFailed
            (Utilities|Casting|CastToBP_StatueRoom _array_element_4
              (:then
                _)
              (:CastFailed
                (Utilities|Casting|CastToBP_LootRoom _array_element_4
                  (:then
                    _)
                  (:CastFailed
                    (Utilities|Casting|CastToBP_EnemyRoom _array_element_4)))))))))
    (Components|StaticMesh|SetStaticMesh (Variables|Default|GetLeftWall) "/Game/Blueprints/Dungeon/OpenWallMesh.OpenWallMesh")))