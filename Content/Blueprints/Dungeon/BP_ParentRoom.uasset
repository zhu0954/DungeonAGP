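; Base dungeon room actor that opens its walls where corridors adjoin it.
; Its Corridor function checks each of the four wall colliders for overlapping BP_ParentRoom actors and casts them to BP_Corridor.
; A corridor hit swaps that side's wall to the open wall mesh.
; The event graph and construction script are empty, so nothing in this graph calls the function.
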(event EventBeginPlay)

(event Collision|EventActorBeginOverlap
  (params (OtherActor :type Actor%20Object%20Reference)))

(event EventTick
  (params (DeltaSeconds :type Float%20%28single-precision%29)))

(fn ConstructionScript)

(fn Corridor
  (for _array_element (Collision|GetOverlappingActors (Variables|Default|GetFrontWallCollider) "BP_ParentRoom_C" :!class /Script/Engine.PrimitiveComponent)
    (Utilities|Casting|CastToBP_Corridor _array_element)
    (Components|StaticMesh|SetStaticMesh (Variables|Default|GetFrontWall) "/Game/Blueprints/Dungeon/OpenWallMesh.OpenWallMesh"))
  (for _array_element_2 (Collision|GetOverlappingActors (Variables|Default|GetLeftWallCollider) "BP_ParentRoom_C" :!class /Script/Engine.PrimitiveComponent)
    (Utilities|Casting|CastToBP_Corridor _array_element_2)
    (Components|StaticMesh|SetStaticMesh (Variables|Default|GetLeftWall) "/Game/Blueprints/Dungeon/OpenWallMesh.OpenWallMesh"))
  (for _array_element_3 (Collision|GetOverlappingActors (Variables|Default|GetBackWallCollider) "BP_ParentRoom_C" :!class /Script/Engine.PrimitiveComponent)
    (Utilities|Casting|CastToBP_Corridor _array_element_3)
    (Components|StaticMesh|SetStaticMesh (Variables|Default|GetBackWall) "/Game/Blueprints/Dungeon/OpenWallMesh.OpenWallMesh"))
  (for _array_element_4 (Collision|GetOverlappingActors (Variables|Default|GetRightWallCollider) "BP_ParentRoom_C" :!class /Script/Engine.PrimitiveComponent)
    (Utilities|Casting|CastToBP_Corridor _array_element_4)
    (Components|StaticMesh|SetStaticMesh (Variables|Default|GetRightWall) "/Game/Blueprints/Dungeon/OpenWallMesh.OpenWallMesh")))